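; BP_Turtle is a turtle that travels to an EndPoint in one of three movement styles, chosen by its type enum on BeginPlay.
; Type One uses AI SimpleMoveToLocation, while Two and Three lerp from the start location with separate timelines, MoveForvardSimple and MoveFB.
; Each type also records an integer ID in IntType.
; Tick watches for arrival within a small tolerance, then plays a 2D sound and destroys the actor.
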(event `self.ReceiveTick`
  (params (DeltaSeconds :type "Float (single-precision)"))
  (`|ExecutionSequence`
    (:`then_0`
      (if true
        _))
    (:`then_1`
      (if (== (`self.K2_GetActorLocation`) (`self.EndPoint`) :`ErrorTolerance` 1.0)
        (`GameplayStatics.PlaySound2D` null 1.0 1.0 0.0 null null)
        (`self.K2_DestroyActor`)))))

(event `self.ReceiveBeginPlay`
  (switch `/Game/TestTack/Structures/E_TypeOfButton` (`self.TypeOfTurrtle`)
    (:`NewEnumerator0`
      (set `self.IntType` 0)
      (`self.MoveFirst`))
    (:`NewEnumerator1`
      (set `self.IntType` 1)
      (set `self.StartPoint` (`self.K2_GetActorLocation` self))
      (bind (_direction _newtrack_0) (`Timeline|Move ForvardSimple`)
        (:`Update`
          (`self.K2_SetActorRelativeLocation` self (`KismetMathLibrary.VLerp` (`self.StartPoint`) (`self.EndPoint`) _newtrack_0) false false))))
    (:`NewEnumerator2`
      (set `self.IntType` 2)
      (set `self.StartPoint` (`self.K2_GetActorLocation` self))
      (bind (_direction_2 _newtrack_0_2) (`Timeline|MoveFB`)
        (:`Update`
          (`self.K2_SetActorRelativeLocation` self (`KismetMathLibrary.VLerp` (`self.StartPoint`) (`self.EndPoint`) _newtrack_0_2) false false))))))

(fn `MoveFirst`
  (`AIBlueprintHelperLibrary.SimpleMoveToLocation` (`AIBlueprintHelperLibrary.GetAIController` self) (`self.EndPoint`)))

(fn `UserConstructionScript`)