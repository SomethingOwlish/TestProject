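; Button actor that spawns a turtle from a nest when the player character overlaps its Cube.
; On BeginPlay it maps its Type (One, Two or Three) to an integer index.
; On overlap it gets all BP_Nest actors and calls SpawnTurtle with its Type on the one at that index.
; Nest pairing relies on the order GetAllActorsOfClass returns, and a trailing switch on Type has no logic attached.
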(event `self.ReceiveBeginPlay`
  (switch `/Game/TestTack/Structures/E_TypeOfButton` (`self.Type`)
    (:`NewEnumerator0`
      (set `self.IntegersByType` 0))
    (:`NewEnumerator1`
      (set `self.IntegersByType` 1))
    (:`NewEnumerator2`
      (set `self.IntegersByType` 2))))

(event `self.ReceiveActorBeginOverlap`
  (params (OtherActor :type "Actor Object Reference")))

(event `self.Cube.OnComponentBeginOverlap`
  (params (OverlappedComponent :type "PrimitiveComponent Object Reference") (OtherActor :type "Actor Object Reference") (OtherComp :type "PrimitiveComponent Object Reference") (OtherBodyIndex :type Integer) (bFromSweep :type Boolean) (SweepResult :type "HitResult Structure (by ref)"))
  (if (== OtherActor (`GameplayStatics.GetPlayerCharacter` 0))
    (bind _outactors (`GameplayStatics.GetAllActorsOfClass` "/Game/TestTack/Blueprints/BP_Nest.BP_Nest_C"))
    (bind _output_get (set `self.All Actors` _outactors))
    (`/Game/TestTack/Blueprints/BP_Nest.SpawnTurtle` (`|GetArrayItem` _output_get (`self.IntegersByType`)) (`self.Type`))
    (switch `/Game/TestTack/Structures/E_TypeOfButton` (`self.Type`))))

(fn `UserConstructionScript`)